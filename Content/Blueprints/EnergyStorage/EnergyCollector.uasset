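; EnergyCollector is an overlap zone actor that controls when the player is allowed to store energy.
; Begin and end overlap events set a flag for Player_Character subclasses, and leaving also clears CanStoreEnergy on BPPlayer_Character.
; While the flag is set, Tick enables CanStoreEnergy whenever the player is neither firing nor playing the wormhole timeline.
; Tick never clears CanStoreEnergy, so it stays enabled until overlap ends unless changed elsewhere.
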(event `self.ReceiveActorBeginOverlap`
  (params (OtherActor :type "Actor Object Reference"))
  (if (`KismetMathLibrary.ClassIsChildOf` (`GameplayStatics.GetObjectClass` OtherActor) "/Script/EL.Player_Character")
    (set `self.overlappingWithPlayer` true)))

(event `self.ReceiveActorEndOverlap`
  (params (OtherActor :type "Actor Object Reference"))
  (if (`KismetMathLibrary.ClassIsChildOf` (`GameplayStatics.GetObjectClass` OtherActor) "/Script/EL.Player_Character")
    (bind _asbpplayer_character (cast `/Game/Blueprints/Player/BPPlayer_Character` OtherActor))
    (if (`/Game/Blueprints/Player/BPPlayer_Character.canStoreEnergy` _asbpplayer_character)
      (set `/Game/Blueprints/Player/BPPlayer_Character.canStoreEnergy` false _asbpplayer_character))
    (set `self.overlappingWithPlayer` false)))

(event `self.ReceiveTick`
  (params (DeltaSeconds :type "Float (single-precision)"))
  (if (`self.overlappingWithPlayer`)
    (bind _asbpplayer_character (cast `/Game/Blueprints/Player/BPPlayer_Character` (stale `self.ReceiveActorBeginOverlap` OtherActor)))
    (if (`/Game/Blueprints/Player/BPPlayer_Character.isFiring` _asbpplayer_character)
      _
      (elif (not (`/Game/Blueprints/Player/BPPlayer_Character.WormholeTimelinePlaying` _asbpplayer_character))
        (set `/Game/Blueprints/Player/BPPlayer_Character.canStoreEnergy` true _asbpplayer_character)))))

(fn `UserConstructionScript`)