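; Player character Blueprint with a hold-to-fire wormhole that pulls in and collects Collectables for Energy, or banks Energy when storing is allowed.
; A timeline plays and reverses with firing, scaling wormhole material parameters, sound volume, fog attraction and two collision spheres.
; The magnet sphere pulls physics components inward; past half open, collected actors add Energy and play timed-combo sounds.
; Tick feeds player position to the Niagara fog parameter collection.
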(event `InputAction|Fire`
  (params (Key :type "Key Structure"))
  (:`Pressed`
    (set `self.isFiring` true)
    (if (`self.canStoreEnergy`)
      (set `self.TotalStoredEnergy` (+ (`self.TotalStoredEnergy`) (`self.Energy`)))
      (set `self.Energy` 0.0)))
  (:`Released`
    (set `self.isFiring` false)))

(event `self.ReceiveTick`
  (params (DeltaSeconds :type "Float (single-precision)"))
  (bind _collectcombo (`self.CollectCombo`))
  (bind _magnetcollision (`self.MagnetCollision`))
  (bind _wormholecollision (`self.WormholeCollision`))
  (bind _wormholecollectsfx (`self.WormholeCollectSFX`))
  (bind _returnvalue (`NiagaraFunctionLibrary.GetNiagaraParameterCollection` "/Game/Particles/FogParticle/NPC_Fog_parameters.NPC_Fog_parameters"))
  (`NiagaraParameterCollectionInstance.SetVectorParameter` _returnvalue "PlayerPosition" (`self.K2_GetActorLocation`))
  (if (`self.isFiring`)
    (if (not (`self.canStoreEnergy`))
      (bind (_direction _wormholefloat) (`Timeline|WormholeTimeline` :!label _label)
        (:`Update`
          (if (> _wormholefloat 0.0)
            (set `self.WormholeTimelinePlaying` true)
            (else
              (set `self.WormholeTimelinePlaying` false)))
          (`KismetMaterialLibrary.SetScalarParameterValue` "/Game/Materials/Wormhole_Ability/MPC_Wormhole.MPC_Wormhole" "WormholeOpacity" _wormholefloat)
          (`KismetMaterialLibrary.SetScalarParameterValue` "/Game/Materials/Wormhole_Ability/MPC_Wormhole.MPC_Wormhole" "Radius" _wormholefloat)
          (`AudioComponent.SetVolumeMultiplier` (`self.WormholeSFX`) _wormholefloat)
          (bind _returnvalue_2 (`NiagaraFunctionLibrary.GetNiagaraParameterCollection` "/Game/Particles/FogParticle/NPC_Fog_parameters.NPC_Fog_parameters"))
          (`NiagaraParameterCollectionInstance.SetVectorParameter` _returnvalue_2 "BlackholePosition" (`SceneComponent.K2_GetComponentLocation` (`self.Wormhole`)))
          (`NiagaraParameterCollectionInstance.SetFloatParameter` _returnvalue_2 "BlackholeStrength" (* _wormholefloat (`self.MaxSmokeAttraction`)))
          (bind _returnvalue_3 (* (`self.MaxCollisionSize`) _wormholefloat))
          (`SphereComponent.SetSphereRadius` _wormholecollision _returnvalue_3 true)
          (`SphereComponent.SetSphereRadius` _magnetcollision (* _returnvalue_3 3.0) true)
          (for _array_element (`PrimitiveComponent.GetOverlappingComponents` _magnetcollision)
            (if (`SceneComponent.IsSimulatingPhysics` _array_element "None")
              (`PrimitiveComponent.AddRadialForce` _array_element (`SceneComponent.K2_GetComponentLocation` (`self.Wormhole`)) (`SphereComponent.GetScaledSphereRadius` _magnetcollision) -1000.0 "RIF_Constant" true))
            (if (>= _wormholefloat 0.5)
              (`KismetMaterialLibrary.SetVectorParameterValue` "/Game/Materials/Wormhole_Ability/MPC_Wormhole.MPC_Wormhole" "CustomPos" (`KismetMathLibrary.Conv_VectorToLinearColor` (`SceneComponent.K2_GetComponentLocation` (`self.Wormhole`))))
              (`ActorComponent.Activate` (`self.PS_Wormhole`) false)
              (bind _ascollectable (cast `/Game/Blueprints/WormholeCollectables/Collectable` (`|GetArrayItem` (`PrimitiveComponent.GetOverlappingActors` _wormholecollision "/Game/Blueprints/WormholeCollectables/Collectable.Collectable_C"))))
              (if (< _collectcombo (`self.CollectComboMax`))
                (`/Engine/EditorBlueprintResources/StandardMacros.IncrementInt` _collectcombo
                  (:`  `
                    _)))
              (`KismetSystemLibrary.K2_SetTimer` null "ResetCollectCombo" 1.5)
              (set `self.Energy` (+ (`/Game/Blueprints/WormholeCollectables/Collectable.Value` _ascollectable) (`self.Energy`)))
              (`self.K2_DestroyActor` _ascollectable)
              (switch `int` (`self.CollectCombo`)
                (:`Default`
                  (`AudioComponent.SetSound` _wormholecollectsfx "/Game/Audio/SFX/PlayerSFX/CollectionSFX/collect_base.collect_base" :!label _label_2))
                (:`0`
                  (goto _label_2))
                (:`1`
                  (`AudioComponent.SetSound` _wormholecollectsfx "/Game/Audio/SFX/PlayerSFX/CollectionSFX/collect_sfx_combo1.collect_sfx_combo1"))
                (:`2`
                  (`AudioComponent.SetSound` _wormholecollectsfx "/Game/Audio/SFX/PlayerSFX/CollectionSFX/collect_sfx_combo2.collect_sfx_combo2"))
                (:`3`
                  (`AudioComponent.SetSound` _wormholecollectsfx "/Game/Audio/SFX/PlayerSFX/CollectionSFX/collect_sfx_combo3.collect_sfx_combo3"))
                (:`4`
                  (`AudioComponent.SetSound` _wormholecollectsfx "/Game/Audio/SFX/PlayerSFX/CollectionSFX/collect_sfx_combo4.collect_sfx_combo4"))
                (:`5`
                  (`AudioComponent.SetSound` _wormholecollectsfx "/Game/Audio/SFX/PlayerSFX/CollectionSFX/collect_sfx_combo5.collect_sfx_combo5"))
                (:`6`
                  (`AudioComponent.SetSound` _wormholecollectsfx "/Game/Audio/SFX/PlayerSFX/CollectionSFX/collect_sfx_combo6.collect_sfx_combo6"))
                (:`7`
                  (`AudioComponent.SetSound` _wormholecollectsfx "/Game/Audio/SFX/PlayerSFX/CollectionSFX/collect_sfx_combo7.collect_sfx_combo7"))
                (:`8`
                  (`AudioComponent.SetSound` _wormholecollectsfx "/Game/Audio/SFX/PlayerSFX/CollectionSFX/collect_sfx_combo8.collect_sfx_combo8")))
              (`AudioComponent.Play` _wormholecollectsfx 0.0)
              (else
                (`ActorComponent.Deactivate` (`self.PS_Wormhole`))))))))
    (else
      (goto _label :!via `Reverse`))))

(fn `ResetCollectCombo`
  (set `self.CollectCombo` 0))

(fn `UserConstructionScript`)