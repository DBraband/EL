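; Pusher actor that shoves the player along its Arrow component's forward direction while overlapping it.
; Begin overlap stores the entering actor, even a non-player, and starts pushing if it is a Player_Character; any end overlap stops it.
; Tick moves the stored actor a small fixed step, without sweep or delta-time scaling, so speed depends on frame rate.
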(event `self.ReceiveActorBeginOverlap`
  (params (OtherActor :type "Actor Object Reference"))
  (bind _output_get (set `self.ActorToPush` OtherActor))
  (if (`KismetMathLibrary.ClassIsChildOf` (`GameplayStatics.GetObjectClass` _output_get) "/Script/EL.Player_Character")
    (set `self.bPushing` true)))

(event `self.ReceiveActorEndOverlap`
  (params (OtherActor :type "Actor Object Reference"))
  (set `self.bPushing` false))

(event `self.ReceiveTick`
  (params (DeltaSeconds :type "Float (single-precision)"))
  (bind _actortopush (`self.ActorToPush`))
  (if (`self.bPushing`)
    (`self.K2_SetActorLocation` _actortopush (+ (`self.K2_GetActorLocation` _actortopush) (* (`SceneComponent.GetForwardVector` (`self.Arrow`)) 0.5)) false false)))

(fn `UserConstructionScript`)