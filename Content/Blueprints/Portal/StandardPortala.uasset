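; StandardPortala is a portal actor that shows a render texture on its frame and teleports the player who crosses it.
; BeginPlay sets the target and applies a dynamic M_PortalBase material, whose PortalTexture parameter SetRTT and ClearRTT update.
; While active, Tick tests the first-person camera against the portal area and plane, then asks the portal manager to teleport the player on a crossing.
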(event `self.ReceiveBeginPlay`
  (`self.SetTarget` (`self.PortalTarget`))
  (bind _returnvalue (`KismetMaterialLibrary.CreateDynamicMaterialInstance` "/Game/Materials/Portal/M_PortalBase.M_PortalBase"))
  (bind _output_get (set `self.MaterialInstance` _returnvalue))
  (`PrimitiveComponent.SetMaterial` (`self.portalframe`) 0 _output_get))

(event `self.ClearRTT`
  (`MaterialInstanceDynamic.SetTextureParameterValue` (`self.MaterialInstance`) "PortalTexture" null))

(event `self.SetRTT`
  (params (RenderTexture :type "Texture Object Reference"))
  (`/Engine/EditorBlueprintResources/StandardMacros.IsValid` RenderTexture
    (:`Is Valid`
      (`MaterialInstanceDynamic.SetTextureParameterValue` (`self.MaterialInstance`) "PortalTexture" RenderTexture))))

(event `self.ReceiveTick`
  (params (DeltaSeconds :type "Float (single-precision)"))
  (bind _portalrootcomponent (`self.PortalRootComponent`))
  (if (`self.IsActive`)
    (bind _asplayer_character (cast `Player_Character` (`GameplayStatics.GetPlayerCharacter` 0)))
    (bind _returnvalue (`SceneComponent.K2_GetComponentLocation` (`Player_Character.FirstPersonCameraComponent` _asplayer_character)))
    (bind _returnvalue_2 (`self.IsPointInsideBox` _returnvalue (`self.Portal_Area`)))
    (if _returnvalue_2
      (bind _returnvalue_3 (`self.IsPointCrossingPortal` _returnvalue (`SceneComponent.K2_GetComponentLocation` _portalrootcomponent) (`SceneComponent.GetForwardVector` _portalrootcomponent)))
      (if _returnvalue_3
        (bind _returnvalue_4 (`self.GetPortalManager` _asplayer_character))
        (`PortalManager.RequestTeleportByPortal` _returnvalue_4 self _asplayer_character)))))

(fn `UserConstructionScript`)