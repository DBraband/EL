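; Cube crate collectable for the wormhole collectables set that gives each spawned crate a random color.
; On BeginPlay it runs the parent logic, then creates a dynamic material instance from the mesh's first material and randomizes its HueShift parameter.
; Overlap and tick events are disabled stubs, so any other behavior comes from the parent class.
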(event `self.ReceiveBeginPlay`
  (`parent.ReceiveBeginPlay`)
  (bind _returnvalue (`PrimitiveComponent.CreateDynamicMaterialInstance` (`self.Mesh`) 0 (`|GetArrayItem` (`MeshComponent.GetMaterials` (`self.Mesh`))) "None"))
  (`MaterialInstanceDynamic.SetScalarParameterValue` _returnvalue "HueShift" (`KismetMathLibrary.RandomFloatInRange` 0.0 300.0)))

(fn `UserConstructionScript`
  (`parent.UserConstructionScript`))